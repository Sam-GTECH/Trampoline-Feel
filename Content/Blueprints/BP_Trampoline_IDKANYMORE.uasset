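; Trampoline actor that deforms or tensions its cloth mesh through a material parameter, currently driven by a debug key.
; BeginPlay creates a dynamic material instance on the cloth mesh.
; Each Tick eases the pressure strength toward a target while E is held, or zero when released, and writes it to the PressionSTR scalar.
; Actor overlap only prints a test message.
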(event EventBeginPlay
  (bind _returnvalue (Rendering|Material|CreateDynamicMaterialInstance (Variables|Default|GetClothMesh) 0 0 "None" :!class /Script/Engine.PrimitiveComponent))
  (Variables|Default|SetClothDynamicMaterialInstance _returnvalue))

(event Collision|EventActorBeginOverlap
  (params (OtherActor :type Actor%20Object%20Reference))
  (Development|PrintString "Hello"))

(event EventTick
  (params (DeltaSeconds :type Float%20%28single-precision%29))
  (bind _output_get (Variables|Default|SetCurrentPressureStrength (Math|Interpolation|FInterpTo (Variables|Default|GetCurrentPressureStrength) (select (Variables|Default|GetisPressing) (Variables|Default|GetTargetPressureStrength) 0.0) (Utilities|Time|GetWorldDeltaSeconds) (Variables|Default|GetTensionSpeed))))
  (Rendering|Material|SetScalarParameterValue (Variables|Default|GetClothDynamicMaterialInstance) "PressionSTR" _output_get :!class /Script/Engine.MaterialInstanceDynamic))

(event Input|KeyboardEvents|DebugKeyE
  (params (Key :type Key%20Structure :default "None") (ActionValue :type Input%20Action%20Value%20Structure))
  (:Pressed
    (Variables|Default|SetisPressing true))
  (:Released
    (Variables|Default|SetisPressing false)))

(fn ConstructionScript)