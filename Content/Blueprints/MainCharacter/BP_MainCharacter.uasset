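; Player character with camera-relative ZQSD movement, mouse look and a jump boosted by trampolines.
; Per-key gates feed movement each Tick, though backward input is disconnected; trampoline jump power scales with center distance and clamped last velocity.
; Tick also tracks landings, widens FOV with height offset from last landing, and moves the camera root vertically with a damped spring tuned separately for above and below.
; Earlier camera experiments remain, unused.
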(event EventBeginPlay
  (Variables|CamEffect=JumpHeightLenght|SetInitialZ (.z (Transformation|GetActorLocation)))
  (Variables|CamEffect=JumpHeightLenght|SetTargetArmLengthDefault (Variables|/Script/Engine.SpringArmComponent|GetTargetArmLength (Variables|Default|GetSpringArm)))
  (Variables|CamEffect=JumpHeightLenght|SetCameraFOVDefault (Variables|/Script/Engine.CameraComponent|GetFieldOfView (Variables|Default|GetCamera)))
  (Variables|ElasticCam2.0|SetLastPlayerZ (.z (Transformation|GetActorLocation)))
  (Variables|ElasticCam2.0|SetCameraRootZ (.z (Transformation|GetWorldLocation (Variables|Default|GetCameraRoot))))
  (Variables|ElasticCam2.0|SetCameraBaseOffsetZ (- (Variables|ElasticCam2.0|GetCameraRootZ) (Variables|ElasticCam2.0|GetLastPlayerZ)))
  (Variables|LookAround|SetInitialRotation (Variables|/Script/Engine.SceneComponent|GetRelativeRotation (Variables|Default|GetCamera))))

(event Collision|EventActorBeginOverlap
  (params (OtherActor :type Actor%20Object%20Reference)))

(event EventOnLanded
  (params (Hit :type Hit%20Result%20Structure%20%28by%20ref%29))
  ;[0.15 0.15 0.15 0.5] Reset Initial Z
  (Variables|CamEffect=JumpHeightLenght|SetInitialZ (.z (Transformation|GetActorLocation))))

(event EventTick
  (params (DeltaSeconds :type Float%20%28single-precision%29))
  (Utilities|FlowControl|Sequence
    (:then_0
      (|ZQSDMovement :!label _label))
    (:then_1
      (goto _label Enter2))
    (:then_2
      (goto _label Enter3))
    (:then_3
      (goto _label Enter4))
    (:then_4
      (|UpdateGroundedLandedInfos))
    (:then_6
      (|FovChange))
    (:then_7
      (|ElasticCameraFollowing DeltaSeconds DeltaSeconds))
    (:then_18
      (Utilities|FlowControl|Sequence
        (:then_4
          (Variables|JumpMecanicsFeatures|SetLastVelocity (Transformation|GetVelocity)))))))

(event Input|KeyboardEvents|SpaceBar
  (params (Key :type Key%20Structure :default "None"))
  ;[0.15 0.15 0.15 0.5] Basic Jump
)

(event Input|KeyboardEvents|SpaceBar
  (params (Key :type Key%20Structure :default "None"))
  (:Pressed
    (CallFunction|JumpCharacter)))

(fn ConstructionScript)

(fn IsonTrampoline
  (bind _usedtrampoline (Variables|JumpMecanicsFeatures|GetUsedTrampoline))
  (return (Utilities|IsValid _usedtrampoline) _usedtrampoline))

(fn CalculateTrampolinePower
  (return (* (Variables|Jump|GetTrampolineBaseJumpStrenght) (Default|GetDistancefromCenterMap (Variables|JumpMecanicsFeatures|GetUsedTrampoline) 2.0 0.0) (Math|Float|Clamp(Float) (Math|Float|Absolute(Float) (Math|Vector|VectorLength (Variables|JumpMecanicsFeatures|GetLastVelocity))) 0.5 1.5))))

(fn GetMouvementScale
  (if (Variables|Jump|GetIsGrounded)
    (return 1.0)
    (else
      (return 1e+02))))

(fn JumpCharacter
  (bind (_ison _trampoline) (CallFunction|IsonTrampoline))
  (Development|PrintString (Utilities|GetDisplayName _trampoline) true true "(R=1.000000,G=0.660000,B=1.000000,A=1.000000)")
  (if _ison
    (LocalVariables|SetJumpPower (CallFunction|CalculateTrampolinePower))
    (else
      (LocalVariables|SetJumpPower (Variables|Jump|GetBasicJumpStrenght))))
  (if (Variables|Jump|GetIsGrounded)
    (Development|PrintString (Utilities|String|ToString(Float) (LocalVariables|GetJumpPower)) true true "(R=1.000000,G=1.000000,B=1.000000,A=1.000000)")
    (Character|LaunchCharacter (Math|Vector|MakeVector 0.0 0.0 (LocalVariables|GetJumpPower)) false false)))

(event Input|KeyboardEvents|Z
  (params (Key :type Key%20Structure))
  (:Pressed
    (Utilities|FlowControl|Gate true) ; enters at Open
  )
  (:Released
    (Utilities|FlowControl|Gate true) ; enters at Close
  ))

(event Input|KeyboardEvents|S
  (params (Key :type Key%20Structure))
  (:Pressed
    (Utilities|FlowControl|Gate true) ; enters at Open
  )
  (:Released
    (Utilities|FlowControl|Gate true) ; enters at Close
  ))

(event Input|KeyboardEvents|D
  (params (Key :type Key%20Structure))
  (:Pressed
    (Utilities|FlowControl|Gate true) ; enters at Open
  )
  (:Released
    (Utilities|FlowControl|Gate true) ; enters at Close
  ))

(event Input|KeyboardEvents|Q
  (params (Key :type Key%20Structure))
  (:Pressed
    (Utilities|FlowControl|Gate true) ; enters at Open
  )
  (:Released
    (Utilities|FlowControl|Gate true) ; enters at Close
  ))

(event Input|MouseEvents|MouseX
  (params (AxisValue :type Float%20%28single-precision%29))
  (bind _initialrotation (Variables|LookAround|GetInitialRotation))
  (Variables|LookAround|SetCurrentYaw (+ AxisValue (Variables|LookAround|GetCurrentYaw)))
  (Pawn|SetControlRotation (Pawn|GetController) (Math|Rotator|MakeRotator (.roll _initialrotation) (+ (.pitch _initialrotation) (Variables|LookAround|GetCurrentPitch)) (+ (.yaw _initialrotation) (Variables|LookAround|GetCurrentYaw)))))

(event Input|MouseEvents|MouseY
  (params (AxisValue :type Float%20%28single-precision%29))
  (bind _initialrotation (Variables|LookAround|GetInitialRotation))
  (Variables|LookAround|SetCurrentPitch (Math|Float|Clamp(Float) (+ (* AxisValue 1.0) (Variables|LookAround|GetCurrentPitch)) -3e+01 25.0))
  (Pawn|SetControlRotation (Pawn|GetController) (Math|Rotator|MakeRotator (.roll _initialrotation) (+ (.pitch _initialrotation) (Variables|LookAround|GetCurrentPitch)) (+ (.yaw _initialrotation) (Variables|LookAround|GetCurrentYaw)))))