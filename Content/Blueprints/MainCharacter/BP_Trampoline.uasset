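; Trampoline actor that registers itself as the main character's UsedTrampoline on overlap and clears it when the overlap ends.
; Overlap begin and end also fire the get-on and get-off dispatchers and print debug messages.
; GetDistanceFromCenter maps player distance to an unclamped 0–100 scale using the actor's XY scale, and GetDistanceFromCenterMap remaps it to a given range.
; Tick prints that distance while a player is on it.
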(event EventBeginPlay)

(event Collision|EventActorBeginOverlap
  (params (OtherActor :type Actor%20Object%20Reference))
  (bind _asbp_main_character_trampoline (Utilities|Casting|CastToBP_MainCharacter_trampoline OtherActor))
  (bind _output_get (Variables|Default|SetPlayerReference _asbp_main_character_trampoline))
  (Variables|/Game/Blueprints/MainCharacter/BP_MainCharacter_trampoline.BP_MainCharacter_trampoline_C|SetUsedTrampoline _output_get self)
  (Development|PrintString "jumping")
  (Default|CallOnGetonTrampoline))

(event Collision|EventActorEndOverlap
  (params (OtherActor :type Actor%20Object%20Reference))
  (bind _asbp_main_character_trampoline (Utilities|Casting|CastToBP_MainCharacter_trampoline OtherActor))
  (Variables|Default|SetPlayerReference 0)
  (Variables|/Game/Blueprints/MainCharacter/BP_MainCharacter_trampoline.BP_MainCharacter_trampoline_C|SetUsedTrampoline _asbp_main_character_trampoline 0)
  (Development|PrintString "bye :(")
  (Default|CallOnGetOffTrampoline))

(event EventTick
  (params (DeltaSeconds :type Float%20%28single-precision%29))
  (if (Utilities|IsValid (Variables|Default|GetPlayerReference))
    (Development|PrintString (Utilities|String|Append (Utilities|GetDisplayName self) ": " (Utilities|String|ToString(Float) (CallFunction|GetDistancefromCenter))))))

(fn ConstructionScript)

(fn GetDistancefromCenter
  (bind _returnvalue (Transformation|GetActorScale3D))
  (return (Math|Float|MapRangeUnclamped (Transformation|GetDistanceTo (Variables|Default|GetPlayerReference)) (Variables|Default|GetminCenter) (* (/ (+ (.x _returnvalue) (.y _returnvalue)) 2e+01) (Variables|Default|GetmaxCenter)) 0.0 1e+02)))

(fn GetDistancefromCenterMap
  (params (Min :type Float%20%28double-precision%29) (Max :type Float%20%28double-precision%29))
  (return (Math|Float|MapRangeUnclamped (CallFunction|GetDistancefromCenter) 0.0 1e+02 Min Max)))