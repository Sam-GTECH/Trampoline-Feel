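; Trampoline actor that catches BP_MainCharacter on sufficiently fast downward overlap and relaunches it after a short absorb window.
; During absorption it disables collision and lowers gravity, then matches buffered jump presses against a window around impact.
; Launch power multiplies curved boosts for jump height, centrality and timing, with HUD feedback and sound.
; Cloth material pressure is driven only by debug key E; several unused legacy paths remain.
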(event Custom|OnAbsorbFinished
  (bind _timingkey (Variables|Timing|GetTimingKey))
  (Utilities|FlowControl|Sequence
    (:then_0
      (|SetVelocity2)
      (Utilities|Time|SetTimerbyEvent (delegate Custom|OnReactivateCollision) 0.2))
    (:then_1
      (Variables|Timing|SetisAbsorbing_state false)
      (Variables|Timing|SetLastValidDelta (.y (Variables|Timing|GetTimingWindowInputPlage)))
      (for _array_element (Variables|/Game/Blueprints/MainCharacter/BP_MainCharacter.BP_MainCharacter_C|GetJumpPressTimes (Variables|Common|GetPlayerReference))
        (Variables|Timing|SetOnAbsorbFinished_CurrentJumpPressArrayElement _array_element)
        (if (and (<= (Variables|Timing|GetOnAbsorbFinished_CurrentJumpPressArrayElement) (+ (Variables|Timing|GetLastCollisionTime) (.y (Variables|Timing|GetTimingWindowInputPlage)))) (>= (Variables|Timing|GetOnAbsorbFinished_CurrentJumpPressArrayElement) (- (Variables|Timing|GetLastCollisionTime) (.x (Variables|Timing|GetTimingWindowInputPlage)))))
          (Utilities|Array|Add (Variables|Timing|GetValidPressTimes) (Variables|Timing|GetOnAbsorbFinished_CurrentJumpPressArrayElement))))
      (if (Utilities|Array|IsNotEmpty (Variables|Timing|GetValidPressTimes))
        (Variables|Timing|SetLastValidDelta (- (Utilities|Array|Get(acopy) (Variables|Timing|GetValidPressTimes) (- (Utilities|Array|Length (Variables|Timing|GetValidPressTimes)) 1)) (Variables|Timing|GetLastCollisionTime)))
        (Utilities|Array|Clear (Variables|Timing|GetValidPressTimes))
        (if (Utilities|Array|IsNotEmpty (Variables|/Game/Blueprints/MainCharacter/BP_MainCharacter.BP_MainCharacter_C|GetJumpPressTimes (Variables|Common|GetPlayerReference)))
          (Utilities|Array|Clear (Variables|/Game/Blueprints/MainCharacter/BP_MainCharacter.BP_MainCharacter_C|GetJumpPressTimes (Variables|Common|GetPlayerReference))))))
    (:then_3
      (bind _boost (CallFunction|CalculateFinalLaunchNew))
      (Character|LaunchCharacter (Variables|Common|GetPlayerReference) (Math|Vector|MakeVector 0.0 0.0 _boost) false false))
    (:then_4
      (Default|ShowTimingText (Variables|/Game/Blueprints/MainCharacter/BP_MainCharacter.BP_MainCharacter_C|GetHUD%20Reference (Variables|Common|GetPlayerReference)) (.Value (Utilities|Map|Find (Variables|Timing|GetTimingFeedbackMap_map) _timingkey)) (Math|Conversions|ToLinearColor(Color) (.Value (Utilities|Map|Find (Variables|Timing|GetTimingFeedbackColor) _timingkey)))))
    (:then_5
      (Variables|/Game/Blueprints/MainCharacter/BP_MainCharacter.BP_MainCharacter_C|SetUsedTrampoline (Variables|Common|GetPlayerReference) 0)
      (Variables|Common|SetPlayerReference 0)
      (Audio|PlaySoundatLocation "/Game/Assets/Audio/JumpTrampoline.JumpTrampoline" (Transformation|GetActorLocation) "0, 0, 0" 1.0 1.0 0.0 0 0 0 0))))

(event Custom|OnReactivateCollision
  (|CollideON_2))

(event EventBeginPlay
  (bind _returnvalue (Rendering|Material|CreateDynamicMaterialInstance (Variables|Default|GetClothMesh) 0 0 "None" :!class /Script/Engine.PrimitiveComponent))
  (Variables|Mesh|SetClothDynamicMaterialInstance _returnvalue))

(event Collision|EventActorBeginOverlap
  (params (OtherActor :type Actor%20Object%20Reference))
  (bind _asbp_main_character (Utilities|Casting|CastToBP_MainCharacter OtherActor))
  (bind _output_get (Variables|Common|SetPlayerReference _asbp_main_character))
  (Variables|/Game/Blueprints/MainCharacter/BP_MainCharacter.BP_MainCharacter_C|SetUsedTrampoline _output_get self)
  (if (CallFunction|ShouldTrampolineHandleJumpOld)
    (Utilities|FlowControl|Sequence
      (:then_0
        (|NoCollide)
        (Projectile|SetVelocity))
      (:then_1
        (CallFunction|CalculateHeightBoostNew))
      (:then_2
        (CallFunction|CalculateCentralityBoostNew))
      (:then_3
        (Variables|Timing|SetLastCollisionTime (Utilities|Time|GetGameTimeinSeconds))
        (Variables|Timing|SetisAbsorbing_state true)
        (Utilities|Time|SetTimerbyEvent (delegate Custom|OnAbsorbFinished) (.y (Variables|Timing|GetTimingWindowInputPlage)))))))

(event Collision|EventActorEndOverlap
  (params (OtherActor :type Actor%20Object%20Reference)))

(event EventTick
  (params (DeltaSeconds :type Float%20%28single-precision%29))
  (Utilities|FlowControl|Sequence
    (:then_0
      (bind _output_get (Variables|Mesh|SetCurrentPressureStrength (Math|Interpolation|FInterpTo (Variables|Mesh|GetCurrentPressureStrength) (select (Variables|Mesh|GetisPressing) (Variables|Mesh|GetTargetPressureStrength) 0.0) (Utilities|Time|GetWorldDeltaSeconds) (Variables|Mesh|GetTensionSpeed))))
      (Rendering|Material|SetScalarParameterValue (Variables|Mesh|GetClothDynamicMaterialInstance) "PressionSTR" _output_get :!class /Script/Engine.MaterialInstanceDynamic))))

(event Input|KeyboardEvents|DebugKeyE
  (params (Key :type Key%20Structure :default "None") (ActionValue :type Input%20Action%20Value%20Structure))
  (:Pressed
    (Variables|Mesh|SetisPressing true)
    (Development|PrintString "Hello"))
  (:Released
    (Variables|Mesh|SetisPressing false)))

(fn ConstructionScript)

(fn GetDistancefromCenterDebug
  (return (Math|Float|Lerp 1.0 0.6 (Math|Float|Clamp(Float) (/ (Math|Vector|Distance(Vector) (Transformation|GetActorLocation (Variables|Common|GetPlayerReference)) (Transformation|GetWorldLocation (Variables|Default|GetStaticMesh))) 2e+02)))))

(fn GetClosestTimingKeyforDeltaNew
  (params (Delta :type Float%20%28double-precision%29))
  (LocalVariables|SetDeltaMs Delta)
  (LocalVariables|SetClosestKey -1.0)
  (LocalVariables|SetSmallestDelta 9999.0)
  (bind _keys (Utilities|Map|Keys (Variables|Timing|GetTimingFeedbackMap_map)))
  (for _array_element _keys
    (LocalVariables|SetCurrentKeyElement _array_element)
    (bind _output_get (LocalVariables|SetCurrentDelta (Math|Float|Absolute(Float) (- (LocalVariables|GetCurrentKeyElement) (LocalVariables|GetDeltaMs)))))
    (if (< _output_get (LocalVariables|GetSmallestDelta))
      (LocalVariables|SetSmallestDelta (LocalVariables|GetCurrentDelta))
      (LocalVariables|SetClosestKey (LocalVariables|GetCurrentKeyElement))))
  (return (LocalVariables|GetClosestKey)))

(fn ShouldTrampolineHandleJumpOld
  (bind _playerreference (Variables|Common|GetPlayerReference))
  (return (<= (.z (Variables|/Game/Blueprints/MainCharacter/BP_MainCharacter.BP_MainCharacter_C|GetLastVelocity _playerreference)) (Variables|/Game/Blueprints/MainCharacter/BP_MainCharacter.BP_MainCharacter_C|GetminSpeedForTrampolineJump_old _playerreference))))

(fn StartAbsorbtionOld
  (bind _playerreference (Variables|Common|GetPlayerReference))
  (Variables|AbsorbtionPhase|SetTimeOnLanding (Utilities|Time|GetGameTimeinSeconds))
  (Variables|/Game/Blueprints/MainCharacter/BP_MainCharacter.BP_MainCharacter_C|SetMoveState _playerreference "NewEnumerator1")
  (Variables|AbsorbtionPhase|SetPlayerVelocityOnLanding (Variables|/Game/Blueprints/MainCharacter/BP_MainCharacter.BP_MainCharacter_C|GetLastVelocity _playerreference))
  (Variables|AbsorbtionPhase|SetAbsorbingPhase true)
  (Variables|AbsorbtionPhase|SetAbsorbtionTimer (+ (Variables|AbsorbtionPhase|GetAbsorbtionTimeMax) 0.0))
  (Variables|AbsorbtionPhase|SetAbsorbtionPhaseTime 0.0)
  (Variables|AbsorbtionPhase|SetPlayerPressedAfterLanding false)
  (Variables|AbsorbtionPhase|SetBlockPressedAfterLanding (Variables|/Game/Blueprints/MainCharacter/BP_MainCharacter.BP_MainCharacter_C|GetJumpBuffered_old (Variables|Common|GetPlayerReference))))

(fn CalculateHeightMultOld
  (bind _outvalue (CallFunction|ReverseExpOld (/ (Math|Float|Absolute(Float) (Math|Vector|VectorLength (Variables|AbsorbtionPhase|GetPlayerVelocityOnLanding))) 1e+03) (Variables|Old|GetHeightExpStrenght_old)))
  (return _outvalue))

(fn ReverseExpOld
  (params (InValue :type Float%20%28double-precision%29) (Strenght :type Float%20%28double-precision%29))
  (bind _result (Math|Float|NegateFloat Strenght)
    (:%20%20
      (return (- (Class|KismetSystemLibrary|MakeLiteralInteger 1) (Class|KismetMathLibrary|Exp (* _result InValue)))))))

(fn HandleTimingInputBufferNew
  (bind _playerreference (Variables|Common|GetPlayerReference))
  (LocalVariables|SetLocalDelta (- (Variables|AbsorbtionPhase|GetTimeOnLanding) (Variables|/Game/Blueprints/MainCharacter/BP_MainCharacter.BP_MainCharacter_C|GetLastJumpPressTime_old (Variables|Common|GetPlayerReference))))
  (bind _output_get (LocalVariables|SetApplyJumpPower? (and (Variables|/Game/Blueprints/MainCharacter/BP_MainCharacter.BP_MainCharacter_C|GetJumpBuffered_old _playerreference) (<= (LocalVariables|GetLocalDelta) (Variables|/Game/Blueprints/MainCharacter/BP_MainCharacter.BP_MainCharacter_C|GetJumpBufferDuration_old _playerreference)))))
  (if _output_get
    (Variables|/Game/Blueprints/MainCharacter/BP_MainCharacter.BP_MainCharacter_C|SetJumpBuffered_old (Variables|Common|GetPlayerReference) false)
    (return (LocalVariables|GetApplyJumpPower?) (LocalVariables|GetLocalDelta))
    (else
      (return (LocalVariables|GetApplyJumpPower?) (LocalVariables|GetLocalDelta)))))

(fn CalculateCentralityBoostNew
  (bind _clothmesh (Variables|Default|GetClothMesh))
  (bind _centralitymultiplicatorrange_config (Variables|CentralityFactor|GetCentralityMultiplicatorRange_config))
  (bind (_min _max) (Components|StaticMesh|GetLocalBounds _clothmesh))
  (Variables|CentralityFactor|SetCentralityJumpBoost_calculation (Math|Float|Lerp (.x _centralitymultiplicatorrange_config) (.y _centralitymultiplicatorrange_config) (Math|Float|Power (Math|Float|Clamp(Float) (- 1.0 (/ (Math|Vector|Distance2D(Vector) (Math|Conversions|ToVector2D(Vector) (Transformation|GetActorLocation (Variables|Common|GetPlayerReference))) (Math|Conversions|ToVector2D(Vector) (Transformation|GetWorldLocation (Variables|Default|GetClothMesh)))) (* (/ (- (.x _max) (.x _min)) 2.0) (.x (Transformation|GetWorldScale _clothmesh)))))) (Variables|CentralityFactor|GetCentralityCurve_config))))
  (return))

(fn CalculateHeightBoostNew
  (bind _expectedjumpheightrange_config (Variables|HeightFactor|GetExpectedJumpHeightRange_config))
  (bind _expectedjumpheightrange_config_2 (Variables|HeightFactor|GetExpectedJumpHeightRange_config))
  (bind _heightmultiplicatorrange_config (Variables|HeightFactor|GetHeightMultiplicatorRange_config))
  (LocalVariables|SetClampedJumpHeight (Math|Float|Clamp(Float) (Variables|/Game/Blueprints/MainCharacter/BP_MainCharacter.BP_MainCharacter_C|GetJumpHeight_HeightFactorCalculation (Variables|Common|GetPlayerReference)) (.x _expectedjumpheightrange_config_2) (.y _expectedjumpheightrange_config_2)))
  (LocalVariables|SetHeightAlpha (/ (- (LocalVariables|GetClampedJumpHeight) (.x (Variables|HeightFactor|GetExpectedJumpHeightRange_config))) (- (.y _expectedjumpheightrange_config) (.x _expectedjumpheightrange_config))))
  (LocalVariables|SetHeightAlphaCurved (Math|Float|Power (LocalVariables|GetHeightAlpha) (Variables|HeightFactor|GetHeightCurve_config)))
  (Variables|HeightFactor|SetHeightJumpBoost_calculation (Math|Float|Lerp (.x _heightmultiplicatorrange_config) (.y _heightmultiplicatorrange_config) (LocalVariables|GetHeightAlphaCurved)))
  (return))

(fn CalculateTimingBoostNew
  (bind _timingmultiplicatorrange_config (Variables|Timing|GetTimingMultiplicatorRange_config))
  (LocalVariables|SetAbsLastValidDelta (Math|Float|Absolute(Float) (Variables|Timing|GetLastValidDelta)))
  (Development|PrintString (Utilities|String|Append "Last ABS valid delta " (Utilities|String|ToString(Float) (LocalVariables|GetAbsLastValidDelta))))
  (if (> (Variables|Timing|GetLastValidDelta) 0.0)
    (LocalVariables|SetNormalizedDelta (/ (LocalVariables|GetAbsLastValidDelta) (.y (Variables|Timing|GetTimingWindowInputPlage))))
    (else
      (bind _output_get (LocalVariables|SetNormalizedDelta (/ (LocalVariables|GetAbsLastValidDelta) (.x (Variables|Timing|GetTimingWindowInputPlage)))))))
  (Development|PrintString (Utilities|String|Append "Normalized delta" (Utilities|String|ToString(Float) _output_get)))
  (bind _output_get_2 (LocalVariables|SetCurveValue (Math|Float|Power (- 1.0 (LocalVariables|GetNormalizedDelta)) (Variables|Timing|GetTimingCurve_config))))
  (Development|PrintString (Utilities|String|Append "Alpha : " (Utilities|String|ToString(Float) _output_get_2)))
  (Variables|Timing|SetTimerJumpBoost_calculation (Math|Float|Lerp (.x _timingmultiplicatorrange_config) (.y _timingmultiplicatorrange_config) (LocalVariables|GetCurveValue))))

(fn CalculateFinalLaunchNew
  (CallFunction|CalculateTimingBoostNew)
  (bind _multiplier (CallFunction|GetClosestTimingKeyforDeltaNew (Variables|Timing|GetLastValidDelta)))
  (Variables|Timing|SetTimingKey _multiplier)
  (return (Math|Float|Clamp(Float) (* (* (* (Variables|Common|GetJumpBasePower) (Variables|HeightFactor|GetHeightJumpBoost_calculation)) (Variables|CentralityFactor|GetCentralityJumpBoost_calculation)) (Variables|Timing|GetTimerJumpBoost_calculation)) 0.0 (Variables|Common|GetMaxJump))))

(fn HandlePlayerJumpNew
  (Variables|/Game/Blueprints/MainCharacter/BP_MainCharacter.BP_MainCharacter_C|SetMoveState (Variables|Common|GetPlayerReference) "NewEnumerator0"))