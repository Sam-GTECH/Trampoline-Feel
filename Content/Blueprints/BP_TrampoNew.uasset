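; Trampoline actor that launches BP_MainCharacter upward when it lands on the box trigger with a fast enough downward velocity.
; Launch power combines an exponential saturating curve of normalized fall speed, a falloff by impact distance from the center, and energy retention, scaled by maximum launch power.
; Separately, Tick eases a pressure parameter on the cloth's dynamic material, raised only while the debug E key is held.
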(event OnComponentBeginOverlap(Box)
  (params (OverlappedComponent :type Primitive%20Component%20Object%20Reference) (OtherActor :type Actor%20Object%20Reference) (OtherComp :type Primitive%20Component%20Object%20Reference) (OtherBodyIndex :type Integer) (bFromSweep :type Boolean) (SweepResult :type Hit%20Result%20Structure%20%28by%20ref%29))
  (bind _asbp_main_character (Utilities|Casting|CastToBP_MainCharacter OtherActor))
  (bind _output_get (Variables|Default|SetPlayerReference _asbp_main_character))
  (Variables|Landing|SetLandingImpact (.impactpoint SweepResult))
  (bind _output_get_2 (Variables|Landing|SetLandingVelocity (Transformation|GetVelocity _output_get)))
  (if (<= (.Z (Math|Vector|BreakVector _output_get_2)) (Variables|/Game/Blueprints/MainCharacter/BP_MainCharacter.BP_MainCharacter_C|GetminSpeedForTrampolineJump _output_get))
    (CallFunction|BoostPlayerUp)))

(event EventBeginPlay
  (bind _returnvalue (Rendering|Material|CreateDynamicMaterialInstance (Variables|Default|GetClothMesh) 0 0 "None" :!class /Script/Engine.PrimitiveComponent))
  (Variables|Mesh|SetClothDynamicMaterialInstance _returnvalue))

(event Collision|EventActorBeginOverlap
  (params (OtherActor :type Actor%20Object%20Reference))
  (Development|PrintString (Utilities|GetDisplayName OtherActor)))

(event EventTick
  (params (DeltaSeconds :type Float%20%28single-precision%29))
  (bind _output_get (Variables|Mesh|SetCurrentPressureStrength (Math|Interpolation|FInterpTo (Variables|Mesh|GetCurrentPressureStrength) (select (Variables|Mesh|GetisPressing) (Variables|Mesh|GetTargetPressureStrength) 0.0) (Utilities|Time|GetWorldDeltaSeconds) (Variables|Mesh|GetTensionSpeed))))
  (Rendering|Material|SetScalarParameterValue (Variables|Mesh|GetClothDynamicMaterialInstance) "PressionSTR" _output_get :!class /Script/Engine.MaterialInstanceDynamic))

(event Input|KeyboardEvents|DebugKeyE
  (params (Key :type Key%20Structure :default "None") (ActionValue :type Input%20Action%20Value%20Structure))
  (:Pressed
    (Variables|Mesh|SetisPressing true))
  (:Released
    (Variables|Mesh|SetisPressing false)))

(fn ConstructionScript)

(fn BoostPlayerUp
  (bind _velmult (CallFunction|GetVelocityMult (CallFunction|GetNormalFallSpeed) (Variables|Jump|GetVelocityStrength)))
  (bind _centermult (CallFunction|GetCenterMult))
  (bind _output_get (LocalVariables|SetFinalBoost (* (* _velmult _centermult (Variables|Default|GetEnergyRetention)) (Variables|Jump|GetMaxLaunchPower))))
  (Character|LaunchCharacter (Variables|Default|GetPlayerReference) (Math|Vector|MakeVector 0.0 0.0 _output_get) false false))

(fn GetNormalFallSpeed
  (return (/ (Math|Float|Absolute(Float) (Math|Float|Min(Float) (.z (Variables|Landing|GetLandingVelocity)) 0.0)) (Variables|Jump|GetReferenceFallSpeed))))

(fn GetVelocityMult
  (params (NormalFall :type Float%20%28double-precision%29) (VelocityStrength :type Float%20%28double-precision%29))
  (return (- 1.0 (Class|KismetMathLibrary|Exp (* (* VelocityStrength -1.0) NormalFall)))))

(fn ReverseExp
  (params (InValue :type Float%20%28double-precision%29) (Strenght :type Float%20%28double-precision%29))
  (bind _result (Math|Float|NegateFloat Strenght)
    (:%20%20
      (return (- (Class|KismetSystemLibrary|MakeLiteralInteger 1) (Class|KismetMathLibrary|Exp (* _result InValue)))))))

(fn GetCenterMult
  (return (Math|Float|Lerp 0.7 1.0 (- 1.0 (Math|Float|Clamp(Float) (/ (Math|Vector|Distance(Vector) (Variables|Landing|GetLandingImpact) (Transformation|GetWorldLocation (Variables|Default|GetCenter))) (Variables|Default|GetRadius)))))))