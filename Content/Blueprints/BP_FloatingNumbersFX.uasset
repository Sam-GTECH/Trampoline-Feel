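; Floating number effect actor that displays an integer as a row of Niagara digit systems.
; CreateNumbers spawns one system per character, yawed to player 0's control rotation and offset sideways, with its digit texture loaded synchronously from Numbers.
; Each system is tracked in DigitSystems with a finished-event binding for removal.
; Tick prints the remaining count as debug output and destroys the actor once the list is empty.
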(event Custom|OnDigitSystemDone
  (params (PSystem :type Niagara%20Component%20Object%20Reference))
  (Utilities|Array|RemoveItem (Variables|Default|GetDigitSystems) PSystem))

(event EventBeginPlay)

(event Collision|EventActorBeginOverlap
  (params (OtherActor :type Actor%20Object%20Reference)))

(event EventTick
  (params (DeltaSeconds :type Float%20%28single-precision%29))
  (Development|PrintString (Utilities|String|ToString(Integer) (Utilities|Array|Length (Variables|Default|GetDigitSystems))) true true "(R=1.000000,G=0.104260,B=0.099486,A=1.000000)")
  (if (Utilities|Array|IsEmpty (Variables|Default|GetDigitSystems))
    (Actor|DestroyActor)))

(fn ConstructionScript)

(fn CreateNumbers
  (params (Number :type Integer))
  (for _array_element (Utilities|String|GetCharacterArrayfromString (Utilities|String|ToString(Integer) Number))
    (bind _returnvalue (Niagara|SpawnSystematLocation "/Game/FloatingNumbersFX.FloatingNumbersFX" "0, 0, 0" (Math|Rotator|MakeRotator 0.0 1.8e+02 (.yaw (Pawn|GetControlRotation (Game|GetPlayerController 0) :!class /Script/Engine.Controller)))))
    (bind _output_get (LocalVariables|SetDigitSystemFX _returnvalue))
    (Transformation|AddLocalOffset _output_get (Math|Vector|MakeVector 0.0 (LocalVariables|GetOffset) 0.0) false false)
    (LocalVariables|SetOffset (+ (LocalVariables|GetOffset) 25.0))
    (bind _returnvalue_2 (Utilities|LoadAssetBlocking (Utilities|Array|Get(acopy) (Variables|Default|GetNumbers) (Math|Conversions|ToInteger(Byte) _array_element))))
    (bind _astexture (Utilities|Casting|CastToTexture _returnvalue_2))
    (Niagara|SetTextureObject (LocalVariables|GetDigitSystemFX) "User.TextureDigits" _astexture)
    (Utilities|Array|Add (Variables|Default|GetDigitSystems) (LocalVariables|GetDigitSystemFX))
    (EventDispatchers|BindEventtoOnSystemFinished (LocalVariables|GetDigitSystemFX) (EventDispatchers|CreateEvent :!event Custom|OnDigitSystemDone))))