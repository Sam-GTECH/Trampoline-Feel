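; Player character Blueprint with ZQSD camera-relative movement, a Space jump when grounded, pitch-clamped mouse look and vertical camera effects.
; Each Tick applies gated movement input, updates grounded state, and eases FOV wider with height offset from the last landing.
; A damped spring then drags the camera root's Z after the character, with different stiffness and damping rising versus falling.
; Earlier arm-length, elastic-cam and landing-pitch experiments remain as disconnected, deprecated graphs.
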(event EventBeginPlay
  (Variables|CamEffect=JumpHeightLenght|SetInitialZ (.z (Transformation|GetActorLocation)))
  (Variables|CamEffect=JumpHeightLenght|SetTargetArmLengthDefault (Variables|/Script/Engine.SpringArmComponent|GetTargetArmLength (Variables|Default|GetSpringArm)))
  (Variables|CamEffect=JumpHeightLenght|SetCameraFOVDefault (Variables|/Script/Engine.CameraComponent|GetFieldOfView (Variables|Default|GetCamera)))
  (Variables|ElasticCam2.0|SetLastPlayerZ (.z (Transformation|GetActorLocation)))
  (Variables|ElasticCam2.0|SetCameraRootZ (.z (Transformation|GetWorldLocation (Variables|Default|GetCameraRoot))))
  (Variables|ElasticCam2.0|SetCameraBaseOffsetZ (- (Variables|ElasticCam2.0|GetCameraRootZ) (Variables|ElasticCam2.0|GetLastPlayerZ)))
  (Variables|LookAround|SetInitialRotation (Variables|/Script/Engine.SceneComponent|GetRelativeRotation (Variables|Default|GetCamera))))

(event Collision|EventActorBeginOverlap
  (params (OtherActor :type Actor%20Object%20Reference)))

(event EventOnLanded
  (params (Hit :type Hit%20Result%20Structure%20%28by%20ref%29))
  ;[0.15 0.15 0.15 0.5] Reset Initial Z
  (Variables|CamEffect=JumpHeightLenght|SetInitialZ (.z (Transformation|GetActorLocation))))

(event EventTick
  (params (DeltaSeconds :type Float%20%28single-precision%29))
  (Utilities|FlowControl|Sequence
    (:then_0
      (|ZQSDMovement :!label _label))
    (:then_1
      (goto _label Enter2))
    (:then_2
      (goto _label Enter3))
    (:then_3
      (goto _label Enter4))
    (:then_4
      (|UpdateGroundedLandedInfos))
    (:then_6
      (|FovChange))
    (:then_17
      (|ElasticCameraFollowing DeltaSeconds DeltaSeconds))))

(event Input|KeyboardEvents|SpaceBar
  (params (Key :type Key%20Structure))
  ;[0.15 0.15 0.15 0.5] Basic Jump
  (:Pressed
    (if (Variables|Jump|GetIsGrounded)
      (Character|LaunchCharacter (Math|Vector|MakeVector 0.0 0.0 (Variables|Jump|GetBasicJumpStrenght)) false false))))

(fn ConstructionScript)

(event Input|KeyboardEvents|Z
  (params (Key :type Key%20Structure))
  (:Pressed
    (Utilities|FlowControl|Gate true) ; enters at Open
  )
  (:Released
    (Utilities|FlowControl|Gate true) ; enters at Close
  ))

(event Input|KeyboardEvents|S
  (params (Key :type Key%20Structure))
  (:Pressed
    (Utilities|FlowControl|Gate true) ; enters at Open
  )
  (:Released
    (Utilities|FlowControl|Gate true) ; enters at Close
  ))

(event Input|KeyboardEvents|D
  (params (Key :type Key%20Structure))
  (:Pressed
    (Utilities|FlowControl|Gate true) ; enters at Open
  )
  (:Released
    (Utilities|FlowControl|Gate true) ; enters at Close
  ))

(event Input|KeyboardEvents|Q
  (params (Key :type Key%20Structure))
  (:Pressed
    (Utilities|FlowControl|Gate true) ; enters at Open
  )
  (:Released
    (Utilities|FlowControl|Gate true) ; enters at Close
  ))

(event Input|MouseEvents|MouseX
  (params (AxisValue :type Float%20%28single-precision%29))
  (bind _initialrotation (Variables|LookAround|GetInitialRotation))
  (Variables|LookAround|SetCurrentYaw (+ AxisValue (Variables|LookAround|GetCurrentYaw)))
  (Pawn|SetControlRotation (Pawn|GetController) (Math|Rotator|MakeRotator (.roll _initialrotation) (+ (.pitch _initialrotation) (Variables|LookAround|GetCurrentPitch)) (+ (.yaw _initialrotation) (Variables|LookAround|GetCurrentYaw)))))

(event Input|MouseEvents|MouseY
  (params (AxisValue :type Float%20%28single-precision%29))
  (bind _initialrotation (Variables|LookAround|GetInitialRotation))
  (Variables|LookAround|SetCurrentPitch (Math|Float|Clamp(Float) (+ (* AxisValue 1.0) (Variables|LookAround|GetCurrentPitch)) -3e+01 25.0))
  (Pawn|SetControlRotation (Pawn|GetController) (Math|Rotator|MakeRotator (.roll _initialrotation) (+ (.pitch _initialrotation) (Variables|LookAround|GetCurrentPitch)) (+ (.yaw _initialrotation) (Variables|LookAround|GetCurrentYaw)))))