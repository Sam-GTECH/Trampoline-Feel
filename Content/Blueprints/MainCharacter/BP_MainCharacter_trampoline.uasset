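; Player character for trampoline jumping, with mouse look, gated ZQSD camera-relative movement and boosted airborne input.
; Jumps launch normally on the ground, while a valid trampoline triggers automatic jumps delegated to its HandlePlayerJump.
; Trampoline power combines center distance, last vertical speed and a multiplier; airborne presses are buffered, but the timing-bonus logic is disconnected.
; Tick updates grounded state and stretches the spring arm with height offset from spawn.
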(event EventBeginPlay
  (Utilities|FlowControl|Sequence
    (:then_0
      (Variables|CameraEffect(ZDelta/TargetArmLenght)|SetInitialZ (.z (Transformation|GetActorLocation)))
      (Variables|CameraEffect(ZDelta/TargetArmLenght)|SetTargetArmLengthDefault (Variables|/Script/Engine.SpringArmComponent|GetTargetArmLength (Variables|Default|GetSpringArm))))
    (:then_1
      (bind _outactors (Actor|GetAllActorsOfClass "/Game/Blueprints/BP_Trampoline.BP_Trampoline_C"))
      (for _array_element _outactors
        _))))

(event Collision|EventActorBeginOverlap
  (params (OtherActor :type Actor%20Object%20Reference)))

(event EventTick
  (params (DeltaSeconds :type Float%20%28single-precision%29))
  (Utilities|FlowControl|Sequence
    (:then_0
      (|ZQSDMovement :!label _label))
    (:then_1
      (goto _label Enter2))
    (:then_2
      (goto _label Enter3))
    (:then_3
      (goto _label Enter4))
    (:then_4
      (|UpdateGroundedLandedInfos))
    (:then_5
      (|ZDeltaTargetArmLenghtBasedOnJump))
    (:then_6
      ;[0.15 0.15 0.15 0.5] Auto-Jump
      (if (and (.IsOn (CallFunction|IsonTrampoline)) (Variables|Jump|GetIsGrounded))
        (CallFunction|JumpCharacter)))
    (:then_9
      (Variables|Default|SetLastVelocity (Math|Conversions|ToVector(Float) (.z (Transformation|GetVelocity)))))))

(event EventOnLanded
  (params (Hit :type Hit%20Result%20Structure%20%28by%20ref%29))
  (Development|PrintString "On Landed")
  (if (.IsOn (CallFunction|IsonTrampoline))
    (Development|PrintString "Combo!")))

(event Input|MouseEvents|MouseX
  (params (AxisValue :type Float%20%28single-precision%29))
  (Pawn|Input|AddControllerYawInput AxisValue))

(event Input|MouseEvents|MouseY
  (params (AxisValue :type Float%20%28single-precision%29))
  (Pawn|Input|AddControllerPitchInput (* AxisValue -1.0)))

(event Input|KeyboardEvents|SpaceBar
  (params (Key :type Key%20Structure :default "None"))
  (:Pressed
    (CallFunction|JumpCharacter)))

(fn ConstructionScript)

(fn JumpCharacter
  (bind (_ison _trampoline) (CallFunction|IsonTrampoline))
  (if (Variables|Jump|GetIsGrounded)
    (if (not _ison)
      (Character|LaunchCharacter (Math|Vector|MakeVector 0.0 0.0 (Variables|Jump|GetBasicJumpStrenght)) false false)
      (else
        (Default|HandlePlayerJump _trampoline)))
    (else
      (bind _output_get (Variables|JumpTiming|SetLastJumpPressTime (Utilities|Time|GetGameTimeinSeconds)))
      (Variables|JumpTiming|SetJumpBuffered true)
      (Development|PrintString (Utilities|String|ToString(Float) _output_get) true true "(R=0.000000,G=1.000000,B=0.000000,A=1.000000)"))))

(fn IsonTrampoline
  (bind _usedtrampoline (Variables|Default|GetUsedTrampoline))
  (return (Utilities|IsValid _usedtrampoline) _usedtrampoline))

(fn CalculateTrampolinePower
  (Utilities|FlowControl|Sequence
    (:then_1
      (return (* (Variables|Jump|GetTrampolineBaseJumpStrenght) (Default|GetDistancefromCenterMap (Variables|Default|GetUsedTrampoline) 2.0 0.0) (Math|Float|Clamp(Float) (Math|Float|Absolute(Float) (Math|Vector|VectorLength (Variables|Default|GetLastVelocity))) 0.5 1.5) (LocalVariables|GetMultiplier))))))

(fn GetMouvementScale
  (if (Variables|Jump|GetIsGrounded)
    (return 1.0)
    (else
      (return 1e+02))))

(event Input|KeyboardEvents|Z
  (params (Key :type Key%20Structure))
  (:Pressed
    (Utilities|FlowControl|Gate true) ; enters at Open
  )
  (:Released
    (Utilities|FlowControl|Gate true) ; enters at Close
  ))

(event Input|KeyboardEvents|S
  (params (Key :type Key%20Structure))
  (:Pressed
    (Utilities|FlowControl|Gate true) ; enters at Open
  )
  (:Released
    (Utilities|FlowControl|Gate true) ; enters at Close
  ))

(event Input|KeyboardEvents|D
  (params (Key :type Key%20Structure))
  (:Pressed
    (Utilities|FlowControl|Gate true) ; enters at Open
  )
  (:Released
    (Utilities|FlowControl|Gate true) ; enters at Close
  ))

(event Input|KeyboardEvents|Q
  (params (Key :type Key%20Structure))
  (:Pressed
    (Utilities|FlowControl|Gate true) ; enters at Open
  )
  (:Released
    (Utilities|FlowControl|Gate true) ; enters at Close
  ))